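; Zombie enemy that chases the player, plays attack animations and takes hits until it dies.
; PawnSensing sightings trigger AIMoveTo toward player controller 0, and arrival plays the attack montage behind a CanAttack busy flag, without applying damage.
; ZombieHit decrements HP, pausing movement for a flag-guarded hit reaction.
; At zero HP, a DoOnce death stops movement, plays a montage, then destroys the actor.
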(event `self.ReceiveBeginPlay`
  ;[1 1 1] q
  (set `self.HP` 10))

(event `self.ReceiveTick`
  (params (DeltaSeconds :type "Float (single-precision)")))

(event `self.PawnSensing.OnSeePawn`
  (params (Pawn :type "Pawn Object Reference"))
  ;[1 1 1] 플레이어를 계속 따라다니도록 설정
  (set `self.IsSeeingPlayer?` true)
  (`self.FollowPlayer`)
  (`KismetSystemLibrary.PrintText` "발견이다!!!!!"))

(event `FollowPlayer`
  ;[1 1 1] 이동 노드
  (if (`self.IsSeeingPlayer?`)
    (`|AIMoveTo` self (0.0 0.0 0.0) (`GameplayStatics.GetPlayerController` 0) 100.0
      (:`OnSuccess`
        ;[1 1 1] 공격 노드
        (if (not (`self.canAttack?`))
          (set `self.canAttack?` true)
          (bind _returnvalue (`self.PlayAnimMontage` self "/Game/Zombie/Animation/Zombie_Attack_Montage.Zombie_Attack_Montage" 1.0 "None"))
          (`KismetSystemLibrary.Delay` _returnvalue)
          (set `self.canAttack?` false)
          (`KismetSystemLibrary.PrintText` "공격이다!!!!!"))))
    (else
      (set `self.IsSeeingPlayer?` false))))

(event `Zombie Hit`
  (bind _output_get (set `self.HP` (- (`self.HP`) 1)))
  (if (<= _output_get 0)
    (`self.Zombie Death`)
    (elif (not (`self.isHit?`))
      (set `self.isHit?` true)
      (`CharacterMovementComponent.DisableMovement` (`self.CharacterMovement`))
      (bind _returnvalue (`self.PlayAnimMontage` "/Game/Zombie/Animation/Zombie_Hit_Montage.Zombie_Hit_Montage"))
      (`KismetSystemLibrary.Delay` (+ _returnvalue 0.5))
      (`CharacterMovementComponent.SetMovementMode` (`self.CharacterMovement`) "MOVE_Walking" 0)
      (set `self.isHit?` false))))

(event `Zombie Death`
  (`/Engine/EditorBlueprintResources/StandardMacros.DoOnce` false
    (:`Completed`
      (`CharacterMovementComponent.DisableMovement` (`self.CharacterMovement`))
      (bind _returnvalue (`self.PlayAnimMontage` "/Game/Zombie/Animation/Zombie_Death_Montage.Zombie_Death_Montage"))
      (`KismetSystemLibrary.Delay` _returnvalue)
      (`self.K2_DestroyActor`))))

(fn `UserConstructionScript`)