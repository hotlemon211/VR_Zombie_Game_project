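; Zombie enemy that moves toward the player, punches on arrival and dies after a few bullet hits.
; BeginPlay starts a single AIMoveTo targeting the player controller; success plays the punch montage, then shows the WB_Credits widget, while PawnSensing is unused.
; BP_Bullet overlaps destroy the bullet and reduce HP, causing either a movement-locked hit reaction or a DoOnce death montage, brief WB_Credits1 widget and actor destruction.
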(event `self.ReceiveBeginPlay`
  ;[1 1 1] q
  (set `self.HP` 2)
  (set `self.IsSeeingPlayer?` true)
  (`self.FollowPlayer`))

(event `self.PawnSensing.OnSeePawn`
  (params (Pawn :type "Pawn Object Reference"))
  ;[1 1 1] 플레이어를 계속 따라다니도록 설정
)

(event `FollowPlayer`
  ;[1 1 1] 이동 노드
  (if (`self.IsSeeingPlayer?`)
    (`|AIMoveTo` self (0.0 0.0 0.0) (`GameplayStatics.GetPlayerController` 0) 100.0
      (:`OnSuccess`
        ;[1 1 1] 공격 노드
        (if (not (`self.canAttack?`))
          (set `self.canAttack?` true)
          (bind _returnvalue (`self.PlayAnimMontage` self "/Game/Zombie/NewZombie/punch.punch" 1.0 "None"))
          (`KismetSystemLibrary.Delay` _returnvalue)
          (set `self.canAttack?` false)
          (`KismetSystemLibrary.PrintText` "공격이다!!!!!" false false)
          (bind _returnvalue_2 (`|CreateWidget` "/Game/UI/WB_Credits.WB_Credits_C"))
          (`UserWidget.AddToViewport` _returnvalue_2 0))))
    (else
      (set `self.IsSeeingPlayer?` false))))

(event `Zombie Hit`
  (bind _output_get (set `self.HP` (- (`self.HP`) 1)))
  (if (<= _output_get 0)
    (`self.Zombie Death`)
    (bind _returnvalue (`|CreateWidget` "/Game/UI/WB_Credits1.WB_Credits1_C"))
    (`UserWidget.AddToViewport` _returnvalue 0)
    (`KismetSystemLibrary.Delay` 1.0)
    (`Widget.RemoveFromParent` _returnvalue)
    (elif (not (`self.isHit?`))
      (set `self.isHit?` true)
      (`CharacterMovementComponent.DisableMovement` (`self.CharacterMovement`))
      (bind _returnvalue_2 (`self.PlayAnimMontage` "/Game/Zombie/NewZombie/montage1.montage1"))
      (`KismetSystemLibrary.Delay` (+ _returnvalue_2 0.5))
      (`CharacterMovementComponent.SetMovementMode` (`self.CharacterMovement`) "MOVE_Walking" 0)
      (set `self.isHit?` false))))

(event `Zombie Death`
  (`/Engine/EditorBlueprintResources/StandardMacros.DoOnce` false
    (:`Completed`
      (`CharacterMovementComponent.DisableMovement` (`self.CharacterMovement`))
      (bind _returnvalue (`self.PlayAnimMontage` "/Game/Zombie/NewZombie/deatghmontag.deatghmontag"))
      (`KismetSystemLibrary.Delay` _returnvalue)
      (`self.K2_DestroyActor`))))

(event `self.ReceiveActorBeginOverlap`
  (params (OtherActor :type "Actor Object Reference"))
  (bind _asbp_bullet (cast `/Game/Guns/Guns/Handgun/Blueprints/BP_Bullet` OtherActor))
  (if true
    (`self.Zombie Hit`)
    (`self.K2_DestroyActor` _asbp_bullet)
    (`KismetSystemLibrary.PrintText` "bullet" false false)))

(fn `GameOver_UI`
  (returns (GameOverUI_ON :type Boolean))
  (return false))

(fn `UserConstructionScript`)