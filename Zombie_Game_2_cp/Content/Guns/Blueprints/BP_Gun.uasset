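; BP_Gun is a grabbable, hand-held gun actor with per-hand Enhanced Input trigger handling.
; Left and right shoot actions drive the trigger mesh rotation and the holding hand animation's trigger value.
; Dropping disables input and removes that hand's weapon mapping context.
; The matching grab setup is disconnected from OnGrabbed, and passing the fire threshold does nothing yet.
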(event `self.MainGrabComponent.OnGrabbed`
  ;[0 0 0 1 32] Main Grab
)

(event `self.MainGrabComponent.OnDropped`
  ;[0 0 0 1 32] Main Grab
  (`self.DisableInput` (`GameplayStatics.GetPlayerController` 0))
  (`EnhancedInputSubsystemInterface.RemoveMappingContext` (pcsubsystem `EnhancedInputLocalPlayerSubsystem` (`GameplayStatics.GetPlayerController` 0)) (select `bool` (`|EnumEquality` (`/Game/VRTemplate/Blueprints/GrabComponent.GetHeldByHand` (`self.MainGrabComponent`)) "Left") :`false` "/Game/VRTemplate/Input/IMC_Weapon_Right.IMC_Weapon_Right" :`true` "/Game/VRTemplate/Input/IMC_Weapon_Left.IMC_Weapon_Left" :!type "InputMappingContext Object Reference") (struct)))

(event `EnhancedInput|/Game/VRTemplate/Input/Actions/IA_GunShoot_Left`
  (params (ActionValue :type "Float (double-precision)") (ElapsedSeconds :type "Float (double-precision)") (TriggeredSeconds :type "Float (double-precision)") (InputAction :type "InputAction Object Reference" :default "/Game/VRTemplate/Input/Actions/IA_GunShoot_Left.IA_GunShoot_Left"))
  (:`Triggered`
    (bind _output_get (set `self.Action Value Left` ActionValue))
    (set `/Game/Hands/AB_HandsAnim.TriggerPressedValue` _output_get (`self.Holding Hand Anim`))
    (`SceneComponent.K2_SetRelativeRotation` (`self.Trigger`) (`KismetMathLibrary.RLerp` (struct) (`self.Trigger Final Possible Rotation`) (`self.Action Value Left`)) false false)
    (if (> (`self.Action Value Left`) (`self.Fire Threshold`))
      _))
  (:`Canceled`
    (set `self.Action Value Left` 0.0 :!label _label)
    (set `/Game/Hands/AB_HandsAnim.TriggerPressedValue` 0.0 (`self.Holding Hand Anim`)))
  (:`Completed`
    (goto _label)))

(event `EnhancedInput|/Game/VRTemplate/Input/Actions/IA_GunShoot_Right`
  (params (ActionValue :type "Float (double-precision)") (ElapsedSeconds :type "Float (double-precision)") (TriggeredSeconds :type "Float (double-precision)") (InputAction :type "InputAction Object Reference" :default "/Game/VRTemplate/Input/Actions/IA_GunShoot_Right.IA_GunShoot_Right"))
  (:`Triggered`
    (bind _output_get (set `self.Action Value Right` ActionValue))
    (set `/Game/Hands/AB_HandsAnim.TriggerPressedValue` _output_get (`self.Holding Hand Anim`))
    (`SceneComponent.K2_SetRelativeRotation` (`self.Trigger`) (`KismetMathLibrary.RLerp` (struct) (`self.Trigger Final Possible Rotation`) (`self.Action Value Right`)) false false)
    (if (> (`self.Action Value Right`) (`self.Fire Threshold`))
      _))
  (:`Canceled`
    (set `self.Action Value Right` 0.0 :!label _label_2)
    (set `/Game/Hands/AB_HandsAnim.TriggerPressedValue` 0.0 (`self.Holding Hand Anim`)))
  (:`Completed`
    (goto _label_2)))

(fn `Get Holding Hand Anim`
  (returns (`Holding Hand Anim` :type "/Game/Hands/AB_HandsAnim Object Reference"))
  (bind _maingrabcomponent (`self.MainGrabComponent`))
  (if (`|EnumEquality` (`/Game/VRTemplate/Blueprints/GrabComponent.GetHeldByHand` _maingrabcomponent) "Left")
    (return (`/Game/VRTemplate/Blueprints/GrabComponent.Left Hand Anim` _maingrabcomponent))
    (else
      (return (`/Game/VRTemplate/Blueprints/GrabComponent.Right Hand Anim` _maingrabcomponent)))))

(fn `UserConstructionScript`)